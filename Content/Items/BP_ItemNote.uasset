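; BP_ItemNote is a pickup note item that registers as a quest item and shows its text to the player when collected.
; It overrides PutIntoBackpack to call the parent, add its ItemName to the backpack's quest items, then display TextNote through the MainMenuGameInstance's ShowNote and run AfterUse.
; BeginPlay and construction only call the parent.
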(event `self.ReceiveBeginPlay`
  (`parent.ReceiveBeginPlay`))

(fn `PutIntoBackpack`
  (params (InBackpack :type "/Game/Blueprints/Components/BP_BackpackComponent Object Reference"))
  (`parent.PutIntoBackpack` InBackpack)
  (`/Game/Blueprints/Components/BP_BackpackComponent.AddQuestItem` (`local.InBackpack`) (`self.ItemName`))
  (bind _asmain_menu_game_instance (cast `/Game/Blueprints/MainMenuGameInstance` (`GameplayStatics.GetGameInstance`)))
  (`/Game/Blueprints/MainMenuGameInstance.ShowNote` _asmain_menu_game_instance (`self.TextNote`))
  (`self.AfterUse`))

(fn `UserConstructionScript`
  (`parent.UserConstructionScript`))