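; Interactable keypad that unlocks its linked door when the entered text matches KeypadCode.
; Overlapping characters toggle a text prompt, while interacting blends the view to the keypad camera and enables mouse clicking.
; Child BP_KeypadButton actors receive a keypad reference, with Buttonentered handling digits, backspace, confirm and exit.
; A correct code returns the view to the player, a wrong one resets entry, and LookAtPlayerCamera runs on Tick but is empty.
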(event `self.ReceiveBeginPlay`
  (`SceneComponent.SetVisibility` (`self.TextRender`) false false))

(event `self.ReceiveTick`
  (params (DeltaSeconds :type "Float (single-precision)"))
  (`self.LookAtPlayerCamera`))

(event `self.ReceiveActorBeginOverlap`
  (params (OtherActor :type "Actor Object Reference"))
  (bind _asbp_character_base (cast `/Game/Blueprints/Character/BP_CharacterBase` OtherActor))
  (set `self.CharacterInBox` _asbp_character_base)
  (`SceneComponent.SetVisibility` (`self.TextRender`) true false)
  (set `self.IsLookAtPlayerCamera` true))

(event `self.ReceiveActorEndOverlap`
  (params (OtherActor :type "Actor Object Reference"))
  (bind _asbp_character_base (cast `/Game/Blueprints/Character/BP_CharacterBase` OtherActor))
  (set `self.CharacterInBox` _asbp_character_base)
  (`SceneComponent.SetVisibility` (`self.TextRender`) false false)
  (set `self.IsLookAtPlayerCamera` false))

(event `Button entered`
  (params (Value :type Text) (`Confirmed?` :type Boolean) (Backspace :type Boolean) (ExitBUTTON :type Boolean))
  (if `Confirmed?`
    (`self.Confirmed`)
    (elif Backspace
      (`self.Backspace`)
      (elif ExitBUTTON
        (`self.back`)
        (elif (`self.CanEnter`)
          (`TextRenderComponent.K2_SetText` (`self.EnterCode`) (`KismetTextLibrary.Conv_StringToText` (`KismetStringLibrary.Concat_StrStr` (`KismetTextLibrary.Conv_TextToString` (`TextRenderComponent.Text` (`self.EnterCode`))) (`KismetTextLibrary.Conv_TextToString` Value))))
          (`TextRenderComponent.SetTextRenderColor` (`self.EnterCode`) (make `Color` 255 255 255 255)))))))

(event `Interactable`
  (bind _returnvalue (`GameplayStatics.GetPlayerController` 0))
  (bind _entercode (`self.EnterCode`))
  (`PlayerController.SetViewTargetWithBlend` (`GameplayStatics.GetPlayerController` 0) (`ActorComponent.GetOwner` (`self.Camera`)) 1.0 "VTBlend_Linear" 0.0 false)
  (`self.DisableInput` (`GameplayStatics.GetPlayerController` 0))
  (`SceneComponent.SetVisibility` (`self.TextRender`) false false)
  (set `PlayerController.bShowMouseCursor` true _returnvalue :!label _label)
  (set `PlayerController.bEnableClickEvents` true _returnvalue)
  (set `PlayerController.bEnableMouseOverEvents` true _returnvalue)
  (`TextRenderComponent.K2_SetText` _entercode (`KismetTextLibrary.Conv_StringToText` (`KismetStringLibrary.GetSubstring` (`KismetTextLibrary.Conv_TextToString` "") 0 (`KismetStringLibrary.Len` (`self.KeypadCode`)))))
  (`TextRenderComponent.SetTextRenderColor` _entercode (make `Color` 200 200 200 255))
  (bind _output_get (set `self.ButtonArry` (`|MakeArray` (`self.Button_0`) (`self.Button_1`) (`self.Button_2`) (`self.Button_3`) (`self.Button_4`) (`self.Button_5`) (`self.Button_6`) (`self.Button_7`) (`self.Button_8`) (`self.Button_9`) (`self.Button_backspace`) (`self.Button_Enter`) (`self.Button_Exit`))))
  (for _array_element _output_get
    (bind _asbp_keypad_button (cast `/Game/Items/BP_KeypadButton` (`ChildActorComponent.ChildActor` _array_element)))
    (set `/Game/Items/BP_KeypadButton.KeypadREF` self _asbp_keypad_button)))

(event `Initable`
  (goto _label))

(event `Backspace`
  (bind _entercode (`self.EnterCode`))
  (bind _returnvalue (`KismetTextLibrary.Conv_TextToString` (`TextRenderComponent.Text` _entercode)))
  (`TextRenderComponent.K2_SetText` _entercode (`KismetTextLibrary.Conv_StringToText` (`KismetStringLibrary.GetSubstring` _returnvalue 0 (- (`KismetStringLibrary.Len` _returnvalue) 1)))))

(event `Confirmed`
  (bind _returnvalue (`GameplayStatics.GetPlayerController` 0))
  (bind _returnvalue_2 (`GameplayStatics.GetPlayerController` 0))
  (if (`KismetStringLibrary.EqualEqual_StrStr` (`self.KeypadCode`) (`KismetTextLibrary.Conv_TextToString` (`TextRenderComponent.Text` (`self.EnterCode`))))
    (`TextRenderComponent.K2_SetText` (`self.EnterCode`) "Correct Pasword")
    (set `/Game/Blueprints/DoorTest/BP_DoorWithCode.IsDoorLocked` false (`self.DoorWithCode`))
    (`KismetSystemLibrary.Delay` 0.5)
    (set `PlayerController.bShowMouseCursor` false _returnvalue)
    (set `PlayerController.bEnableClickEvents` false _returnvalue)
    (set `PlayerController.bEnableMouseOverEvents` false _returnvalue)
    (for _array_element (`self.ButtonArry`)
      (bind _asbp_keypad_button (cast `/Game/Items/BP_KeypadButton` (`ChildActorComponent.ChildActor` _array_element)))
      (`/Game/Items/BP_KeypadButton.Reset Button` _asbp_keypad_button))
    (`PlayerController.SetViewTargetWithBlend` (`GameplayStatics.GetPlayerController` 0) (`ActorComponent.GetOwner` (`/Game/Blueprints/Character/BP_CharacterBase.Camera` (cast `/Game/Blueprints/Character/BP_CharacterBase` (`GameplayStatics.GetPlayerPawn` 0) :!pure true))) 1.0 "VTBlend_Linear" 0.0 false)
    (`TextRenderComponent.K2_SetText` (`self.EnterCode`) "")
    (else
      (`TextRenderComponent.K2_SetText` (`self.EnterCode`) "Wrong Pasword")
      (`KismetSystemLibrary.Delay` 0.5)
      (set `PlayerController.bEnableClickEvents` false _returnvalue_2)
      (set `PlayerController.bEnableMouseOverEvents` false _returnvalue_2)
      (for _array_element_2 (`self.ButtonArry`)
        (bind _asbp_keypad_button_2 (cast `/Game/Items/BP_KeypadButton` (`ChildActorComponent.ChildActor` _array_element_2)))
        (`/Game/Items/BP_KeypadButton.Reset Button` _asbp_keypad_button_2))
      (`self.Initable`)
      (set `self.CanEnter` true)
      (`self.EnableInput` (`GameplayStatics.GetPlayerController` 0)))))

(event `back`
  (bind _returnvalue (`GameplayStatics.GetPlayerController` 0))
  (set `PlayerController.bShowMouseCursor` false _returnvalue)
  (set `PlayerController.bEnableClickEvents` false _returnvalue)
  (set `PlayerController.bEnableMouseOverEvents` false _returnvalue)
  (for _array_element (`self.ButtonArry`)
    (bind _asbp_keypad_button (cast `/Game/Items/BP_KeypadButton` (`ChildActorComponent.ChildActor` _array_element)))
    (`/Game/Items/BP_KeypadButton.Reset Button` _asbp_keypad_button))
  (`PlayerController.SetViewTargetWithBlend` (`GameplayStatics.GetPlayerController` 0) (`ActorComponent.GetOwner` (`/Game/Blueprints/Character/BP_CharacterBase.Camera` (cast `/Game/Blueprints/Character/BP_CharacterBase` (`GameplayStatics.GetPlayerPawn` 0) :!pure true))) 1.0 "VTBlend_Linear" 0.0 false)
  (`TextRenderComponent.K2_SetText` (`self.EnterCode`) "")
  (`self.EnableInput` (`GameplayStatics.GetPlayerController` 0)))

(fn `Interact`
  (returns (Success :type Boolean))
  (`self.Interactable`)
  (return true))

(fn `LookAtPlayerCamera`)

(fn `OnRep_KeypadCode`)

(fn `UserConstructionScript`)