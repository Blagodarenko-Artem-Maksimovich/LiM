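; BP_KeypadButton is a single clickable button for an in-game keypad.
; On click it passes its number and its confirm, backspace and exit flags to the referenced keypad's ButtonEntered.
; Cursor hover swaps the button material as a highlight, and both cursor exit and the ResetButton event restore the red default.
; The construction script writes the assigned number onto the button's text.
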(event `self.Button.OnClicked`
  (params (TouchedComponent :type "PrimitiveComponent Object Reference") (ButtonPressed :type "Key Structure"))
  (`/Game/Items/BP_Keypad.Button entered` (`self.KeypadREF`) (`self.ButtonNumber`) (`self.ConfirmButton`) (`self.BackspaceButton`) (`self.ExitButton`)))

(event `self.Button.OnBeginCursorOver`
  (params (TouchedComponent :type "PrimitiveComponent Object Reference"))
  (`PrimitiveComponent.SetMaterial` (`self.Button`) 0 "/Game/Content/Camera/Camera_mat.Camera_mat"))

(event `self.Button.OnEndCursorOver`
  (params (TouchedComponent :type "PrimitiveComponent Object Reference"))
  (`PrimitiveComponent.SetMaterial` (`self.Button`) 0 "/Game/untitled_category/untitled_asset/M_book_red.M_book_red" :!label _label))

(event `Reset Button`
  (goto _label))

(fn `UserConstructionScript`
  (`TextRenderComponent.K2_SetText` (`self.Button_Number`) (`self.ButtonNumber`)))