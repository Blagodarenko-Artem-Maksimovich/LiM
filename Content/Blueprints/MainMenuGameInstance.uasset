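; Game instance that manages the game's UI: main, options and pause menus, a quit-to-main confirmation, a note reader and a timed test widget.
; Events create widgets, mostly cached, and add or remove them, switching input mode, cursor visibility and pause state as needed.
; It also opens the new-game and main menu levels.
; Main menu display branches on an entry counter and uses a delayed, do-once helper to center the cursor.
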(event `Show Options Menu`
  (`/Engine/EditorBlueprintResources/StandardMacros.IsValid` (`self.OptionsMenuWB`)
    (:`Is Valid`
      _)
    (:`Is Not Valid`
      (bind _returnvalue (`|CreateWidget` "/Game/UI/Menus/OptionMenuWB.OptionMenuWB_C" (`GameplayStatics.GetPlayerController` 0)))
      (set `self.OptionsMenuWB` _returnvalue)))
  (`UserWidget.AddToViewport` (`self.OptionsMenuWB`) 0))

(event `Create New Game`
  (`GameplayStatics.OpenLevel` "LevelFlat"))

(event `BackToMenu`
  (bind _returnvalue (`GameplayStatics.GetPlayerController` 0))
  (`Widget.RemoveFromParent` (`self.OptionsMenuWB`))
  (`/Engine/EditorBlueprintResources/StandardMacros.IsValid` (`self.MainMenuWB`)
    (:`Is Valid`
      (bind _returnvalue_2 (`|CreateWidget` "/Game/UI/Menus/MainMenuWB.MainMenuWB_C" _returnvalue)))
    (:`Is Not Valid`
      _))
  (set `self.MainMenuWB` _returnvalue_2)
  (`UserWidget.AddToViewport` (`self.MainMenuWB`) 0)
  (set `PlayerController.bShowMouseCursor` true _returnvalue)
  (`WidgetBlueprintLibrary.SetInputMode_UIOnlyEx` _returnvalue (`self.MainMenuWB`) "LockInFullscreen")
  (`self.Cursor to center`))

(event `Show Pause Menu`
  (bind _returnvalue (`GameplayStatics.GetPlayerController` 0))
  (bind _pausemenuwb (`self.PauseMenuWB`))
  (`/Engine/EditorBlueprintResources/StandardMacros.IsValid` (`self.PauseMenuWB`)
    (:`Is Valid`
      _)
    (:`Is Not Valid`
      (bind _returnvalue_2 (`|CreateWidget` "/Game/UI/Menus/PauseMenuWB.PauseMenuWB_C" _returnvalue))
      (set `self.PauseMenuWB` _returnvalue_2)))
  (`UserWidget.AddToViewport` _pausemenuwb 0)
  (`WidgetBlueprintLibrary.SetInputMode_UIOnlyEx` _returnvalue _pausemenuwb "LockInFullscreen")
  (`GameplayStatics.SetGamePaused` true)
  (set `PlayerController.bShowMouseCursor` true _returnvalue))

(event `Show Main Menu`
  (bind _returnvalue (`GameplayStatics.GetPlayerController` 0))
  (bind _returnvalue_2 (`GameplayStatics.GetPlayerController` 0))
  (`/Engine/EditorBlueprintResources/StandardMacros.IncrementInt` (`self.MMEnter`)
    (:`  `
      (if (== (`self.MMEnter`) 1)
        (`/Engine/EditorBlueprintResources/StandardMacros.IsValid` (`self.MainMenuWB`)
          (:`Is Valid`
            _)
          (:`Is Not Valid`
            (bind _returnvalue_3 (`|CreateWidget` "/Game/UI/Menus/MainMenuWB.MainMenuWB_C" _returnvalue_2))))
        (set `self.MainMenuWB` _returnvalue_3)
        (`UserWidget.AddToViewport` (`self.MainMenuWB`) 0)
        (set `PlayerController.bShowMouseCursor` true _returnvalue_2)
        (`WidgetBlueprintLibrary.SetInputMode_UIOnlyEx` _returnvalue_2 (`self.MainMenuWB`) "LockInFullscreen")
        (`self.Cursor to center`)
        (else
          (`/Engine/EditorBlueprintResources/StandardMacros.IsValid` (`self.MainMenuWB`)
            (:`Is Valid`
              (bind _returnvalue_4 (`|CreateWidget` "/Game/UI/Menus/MainMenuWB.MainMenuWB_C" _returnvalue)))
            (:`Is Not Valid`
              _))
          (set `self.MainMenuWB` _returnvalue_4)
          (`UserWidget.AddToViewport` (`self.MainMenuWB`) 0)
          (set `PlayerController.bShowMouseCursor` true _returnvalue)
          (`WidgetBlueprintLibrary.SetInputMode_UIOnlyEx` _returnvalue (`self.MainMenuWB`) "LockInFullscreen")
          (`self.Cursor to center`))))))

(event `Pause Menu Continue`
  (bind _returnvalue (`GameplayStatics.GetPlayerController` 0))
  (`Widget.RemoveFromParent` (`self.PauseMenuWB`))
  (`GameplayStatics.SetGamePaused` false)
  (`WidgetBlueprintLibrary.SetInputMode_GameOnly` _returnvalue)
  (set `PlayerController.bShowMouseCursor` false _returnvalue))

(event `Back to Main Menu`
  (`/Engine/EditorBlueprintResources/StandardMacros.IsValid` (`self.PauseToMainMenuWB`)
    (:`Is Valid`
      _)
    (:`Is Not Valid`
      (bind _returnvalue (`|CreateWidget` "/Game/UI/Menus/PaustoMainWB.PaustoMainWB_C" (`GameplayStatics.GetPlayerController` 0)))
      (set `self.PauseToMainMenuWB` _returnvalue)))
  (`UserWidget.AddToViewport` (`self.PauseToMainMenuWB`) 0)
  (`Widget.RemoveFromParent` (`self.PauseMenuWB`)))

(event `PauseToMainYes`
  (`GameplayStatics.OpenLevel` "MainMenu"))

(event `PauseToMaineNo`
  (`Widget.RemoveFromParent` (`self.PauseToMainMenuWB`))
  (`self.Pause Menu Continue`))

(event `TESTON`
  (`/Engine/EditorBlueprintResources/StandardMacros.IsValid` (`self.TextWB`)
    (:`Is Valid`
      _)
    (:`Is Not Valid`
      (bind _returnvalue (`|CreateWidget` "/Game/Blueprints/HUD/BPW_Test.BPW_Test_C" (`GameplayStatics.GetPlayerController` 0)))
      (set `self.TextWB` _returnvalue)))
  (`UserWidget.AddToViewport` (`self.TextWB`) 0)
  (`KismetSystemLibrary.Delay` 4.0)
  (`Widget.RemoveFromParent` (`self.TextWB`)))

(event `ShowNote`
  (params (NewText :type Text))
  (bind _returnvalue (`GameplayStatics.GetPlayerController` 0))
  (bind _notewb (`self.NoteWB`))
  (`/Engine/EditorBlueprintResources/StandardMacros.IsValid` (`self.NoteWB`)
    (:`Is Valid`
      _)
    (:`Is Not Valid`
      (bind _returnvalue_2 (`|CreateWidget` "/Game/UI/Menus/NoteWB.NoteWB_C" _returnvalue))
      (set `self.NoteWB` _returnvalue_2)))
  (`UserWidget.AddToViewport` _notewb 0)
  (`/Game/UI/Menus/NoteWB.Set Note` _notewb NewText)
  (`WidgetBlueprintLibrary.SetInputMode_UIOnlyEx` _returnvalue _notewb "LockInFullscreen")
  (set `PlayerController.bShowMouseCursor` true _returnvalue))

(event `Back`
  (bind _returnvalue (`GameplayStatics.GetPlayerController` 0))
  (`Widget.RemoveFromParent` (`self.NoteWB`))
  (`GameplayStatics.SetGamePaused` false)
  (`WidgetBlueprintLibrary.SetInputMode_GameOnly` _returnvalue)
  (set `PlayerController.bShowMouseCursor` false _returnvalue))