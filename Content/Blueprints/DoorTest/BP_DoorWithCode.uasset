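; Interactable door Blueprint that toggles open and closed through Interact when it is ready and unlocked.
; When locked, Interact adds a no-key widget to the viewport instead.
; Unlock and SwitchLock change the lock flag, while Lock is empty.
; Key-index locking, unlock sound, random no-key voice lines and a timer are disconnected, and nothing visible calls Errw to remove the widget.
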(fn `errw`
  (`Widget.RemoveFromParent` (`self.Test`)))

(fn `Interact`
  (returns (Success :type Boolean))
  (locals (L_Backpack :type "/Game/Blueprints/Components/BP_BackpackComponent Object Reference") (L_ItemName :type Name) (L_ItemInc :type Integer) (NewLocalVar :type "SubmixEffectDelaySettings Structure"))
  (if (`self.IsReadyToInteract`)
    (if (not (`self.IsDoorLocked`))
      (if (`self.IsDoorOpen`)
        (`self.CloseDoor`)
        (return true)
        (else
          (`self.OpenDoor`)
          (return true)))
      (else
        (bind _returnvalue (`|CreateWidget` "/Game/Blueprints/HUD/BPW_DoorNoKey.BPW_DoorNoKey_C"))
        (bind _output_get (set `self.Test` _returnvalue))
        (`UserWidget.AddToViewport` _output_get 0)
        (return true)))
    (else
      (return false))))

(fn `Lock`)

(fn `SwitchLock`
  (set `self.IsDoorLocked` (not (`self.IsDoorLocked`))))

(fn `Unlock`
  (set `self.IsDoorLocked` false))

(fn `UserConstructionScript`
  (`parent.UserConstructionScript`))