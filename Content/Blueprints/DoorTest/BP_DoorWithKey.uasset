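; Interactable door that toggles open and closed, or, when locked, requires named quest-item keys from the player's backpack.
; Interact looks up the backpack component on the character in its box and removes each matching key as found, even if the set is incomplete.
; A full set unlocks the door with a sound; otherwise a no-key widget and random voice line play, with a timer set afterward.
; Lock only takes effect when no keys are configured.
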(fn `errw`
  (`Widget.RemoveFromParent` (`self.Test`)))

(fn `Interact`
  (returns (Success :type Boolean))
  (locals (L_Backpack :type "/Game/Blueprints/Components/BP_BackpackComponent Object Reference") (L_ItemName :type Name) (L_ItemInc :type Integer) (NewLocalVar :type "SubmixEffectDelaySettings Structure"))
  (if (`self.IsReadyToInteract`)
    (if (not (`self.IsDoorLocked`))
      (if (`self.IsDoorOpen`)
        (`self.CloseDoor`)
        (return true)
        (else
          (`self.OpenDoor`)
          (return true)))
      (elif (`KismetArrayLibrary.Array_IsValidIndex` (`self.NeededKeysName`))
        (bind _characterinbox (`self.CharacterInBox`)
          (:`then`
            (bind _returnvalue (`self.GetComponentByClass` _characterinbox "/Game/Blueprints/Components/BP_BackpackComponent.BP_BackpackComponent_C"))
            (`/Engine/EditorBlueprintResources/StandardMacros.IsValid` _returnvalue
              (:`Is Valid`
                (set `local.L_Backpack` _returnvalue)
                (for _array_element (`self.NeededKeysName`)
                  (set `local.L_ItemName` _array_element)
                  (if (`BlueprintSetLibrary.Set_Contains` (`/Game/Blueprints/Components/BP_BackpackComponent.QuestItem` (`local.L_Backpack`)) (`local.L_ItemName`))
                    (`/Engine/EditorBlueprintResources/StandardMacros.IncrementInt` (`local.L_ItemInc`)
                      (:`  `
                        (`/Game/Blueprints/Components/BP_BackpackComponent.RemoveQuestItem` (`local.L_Backpack`) (`local.L_ItemName`))))))
                (if (== (`local.L_ItemInc`) (`KismetArrayLibrary.Array_Length` (`self.NeededKeysName`)))
                  (`self.Unlock`)
                  (`GameplayStatics.PlaySoundAtLocation` "/Game/Sounds/DoorEffects/doorhasopened.doorhasopened" (`SceneComponent.K2_GetComponentLocation` (`self.StaticMesh_0`)) (struct) 1.0 1.0 0.0 "/Game/Sounds/TestAudio.TestAudio" null null null)
                  (else
                    (bind _returnvalue_2 (`|CreateWidget` "/Game/Blueprints/HUD/BPW_DoorNoKey.BPW_DoorNoKey_C"))
                    (bind _output_get (set `self.Test` _returnvalue_2))
                    (`UserWidget.AddToViewport` _output_get 0)
                    (`GameplayStatics.PlaySound2D` (select `int` (`KismetMathLibrary.RandomIntegerInRange` 0 3) :`0` "/Game/Sounds/VoiceLines/NoKeyVL/mcnokeyvl1.mcnokeyvl1" :`1` "/Game/Sounds/VoiceLines/NoKeyVL/mcnokeyvl2.mcnokeyvl2" :`2` "/Game/Sounds/VoiceLines/NoKeyVL/mcnokeyvl3.mcnokeyvl3" :`3` "/Game/Sounds/VoiceLines/NoKeyVL/mcnokeyvl4.mcnokeyvl4" :!type "SoundBase Object Reference") 1.0 1.0 0.0 null null)
                    (`KismetSystemLibrary.K2_SetTimerDelegate` (`|CreateDelegate` :!event `errw`) 3.0)
                    (return true))))))
          (:`else`
            (return true)))
        (else
          (return true))))
    (else
      (return false))))

(fn `Lock`
  (if (not (`KismetArrayLibrary.Array_IsValidIndex` (`self.NeededKeysName`)))
    (set `self.IsDoorLocked` true)))

(fn `SwitchLock`
  (set `self.IsDoorLocked` (not (`self.IsDoorLocked`))))

(fn `Unlock`
  (set `self.IsDoorLocked` false))

(fn `UserConstructionScript`
  (`parent.UserConstructionScript`))